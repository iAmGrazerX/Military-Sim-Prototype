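; Base AI controller that runs StateTree logic and reacts to perceiving the player character.
; It starts its StateTree component on BeginPlay, then listens for AI Perception updates about player 0.
; A successful sense sends an AI.Test event into the StateTree, while losing the player prints a debug message and clears focus.
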(event `self.ReceiveBeginPlay`
  (`BrainComponent.StartLogic` (`self.StateTreeAI`)))

(event `self.AIPerception.OnTargetPerceptionUpdated`
  (params (Actor :type "Actor Object Reference") (Stimulus :type "AIStimulus Structure"))
  (if (== (`GameplayStatics.GetPlayerCharacter` 0) Actor)
    (if Stimulus_bSuccessfullySensed
      (`StateTreeComponent.SendStateTreeEvent` (`self.StateTreeAI`) (make `StateTreeEvent` (struct :`TagName` "AI.Test")))
      (else
        (`KismetSystemLibrary.PrintString` "BIDHU GONE WHERE GONE")
        (`self.K2_ClearFocus`)))))

(fn `UserConstructionScript`)