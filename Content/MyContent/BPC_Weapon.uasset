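; Weapon component that draws a debug aim trace for the player's ALS character while aiming with a weapon in hand.
; Each Tick it casts player 0's character, checks rotation mode through the ALS state interface, and confirms a weapon mesh is set.
; It then runs a visibility line trace using Line Trace Location, which computes the muzzle socket and a screen-center point at Range.
; The hit result is unused.
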(event `self.ReceiveTick`
  (params (DeltaSeconds :type "Float (single-precision)"))
  (bind _returnvalue (`GameplayStatics.GetPlayerController` 0))
  (bind (_sizex _sizey) (`PlayerController.GetViewportSize` _returnvalue))
  (bind (_worldposition _worlddirection) (`GameplayStatics.DeprojectScreenToWorld` _returnvalue (`KismetMathLibrary.MakeVector2D` (`KismetMathLibrary.Conv_IntToDouble` (/ _sizex 2)) (`KismetMathLibrary.Conv_IntToDouble` (/ _sizey 2)))))
  ; Casting To Character
  (bind _asals_anim_man_character_bp (cast `/Game/AdvancedLocomotionV4/Blueprints/CharacterLogic/ALS_AnimMan_CharacterBP` (`GameplayStatics.GetPlayerCharacter` 0))
    (:`then`
      (bind _output_get (set `self.Character Ref` _asals_anim_man_character_bp))
      ; Checking Aim State
      (bind (_pawnmovementmode _movementstate _prevmovementstate _movementaction _rotationmode) (message `/Game/AdvancedLocomotionV4/Blueprints/Interfaces/ALS_Character_BPI.BPI_Get_CurrentStates` _output_get))
      (if (`|EnumEquality` _rotationmode "NewEnumerator3")
        ; Checking Weapon in Hand
        (`/Engine/EditorBlueprintResources/StandardMacros.IsValid` (`SkeletalMeshComponent.GetSkeletalMeshAsset` (`/Game/AdvancedLocomotionV4/Blueprints/CharacterLogic/ALS_AnimMan_CharacterBP.SkeletalMesh` (`self.Character Ref`)))
          (:`Is Valid`
            ; Raycasting from Weapon
            (`KismetSystemLibrary.LineTraceSingle` :`Start` (`SceneComponent.GetSocketLocation` (`/Game/AdvancedLocomotionV4/Blueprints/CharacterLogic/ALS_AnimMan_CharacterBP.SkeletalMesh` (`self.Character Ref`)) "muzzle") :`End` (+ _worldposition (* _worlddirection (`self.Range`))) :`TraceChannel` "TraceTypeQuery1" :`DrawDebugType` "ForOneFrame" :`DrawTime` 2.0)))))
    (:`CastFailed`
      (`KismetSystemLibrary.PrintString` "Failed to cast Character BP" true true (struct :`R` 1.0 :`G` 0.02598 :`A` 1.0)))))