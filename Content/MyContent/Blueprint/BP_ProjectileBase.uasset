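; Base projectile actor that damages what it hits, taking speed, gravity, lifetime and damage from ProjectileData.
; Construction applies that data to ProjectileMovement and lifespan; BeginPlay makes Collision ignore the instigator when moving.
; Overlaps pass a one-shot validation macro screening instigator and self, then send damage through BPI_Damageable where implemented and destroy the projectile.
; An Impact function duplicates the validation and damage logic but is not called here.
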(event `self.ReceiveBeginPlay`
  (`PrimitiveComponent.IgnoreActorWhenMoving` (`self.Collision`) (`self.InstigatorActor`) true))

(event `self.Collision.OnComponentBeginOverlap`
  (params (OverlappedComponent :type "PrimitiveComponent Object Reference") (OtherActor :type "Actor Object Reference") (OtherComp :type "PrimitiveComponent Object Reference") (OtherBodyIndex :type Integer) (bFromSweep :type Boolean) (SweepResult :type "HitResult Structure (by ref)"))
  (bind (_projectiledata_speed _projectiledata_gravityscale _projectiledata_lifetime _projectiledata_damage) (break `/Game/MyContent/Struct/ST_ProjectileData` (`self.ProjectileData`)))
  (if (not (`self.HasImpacted`))
    (set `self.HasImpacted` true)
    (if (or (== OtherActor (`self.InstigatorActor`)) (== OtherActor self))
      _
      (elif (`KismetSystemLibrary.DoesImplementInterface` OtherActor "/Game/MyContent/Blueprint/BPI_Damageable.BPI_Damageable_C")
        (message `/Game/MyContent/Blueprint/BPI_Damageable.RecieveDamage` OtherActor _projectiledata_damage (`self.InstigatorActor`) SweepResult)
        (`self.DestroySelf`)
        (else
          (`self.DestroySelf`))))))

(fn `DestroySelf`
  (`self.K2_DestroyActor`))

(fn `Impact`
  (params (`Other Actor` :type "Object Object Reference") (Damage :type "Float (double-precision)") (`Hit Result` :type "HitResult Structure"))
  ; Validation
  (if (`self.HasImpacted`)
    (return)
    (else
      (set `self.HasImpacted` true)
      (if (or (== `Other Actor` (`self.InstigatorActor`)) (== `Other Actor` self))
        (return)
        (elif (`KismetSystemLibrary.DoesImplementInterface` `Other Actor` "/Game/MyContent/Blueprint/BPI_Damageable.BPI_Damageable_C")
          (message `/Game/MyContent/Blueprint/BPI_Damageable.RecieveDamage` `Other Actor` Damage (`self.InstigatorActor`) `Hit Result`))))))

(fn `UserConstructionScript`
  (bind (_projectiledata_speed _projectiledata_gravityscale _projectiledata_lifetime) (break `/Game/MyContent/Struct/ST_ProjectileData` (`self.ProjectileData`)))
  (bind _projectilemovement (`self.ProjectileMovement`))
  (set `ProjectileMovementComponent.InitialSpeed` _projectiledata_speed _projectilemovement)
  (set `ProjectileMovementComponent.MaxSpeed` _projectiledata_speed _projectilemovement)
  (set `ProjectileMovementComponent.ProjectileGravityScale` _projectiledata_gravityscale _projectilemovement)
  (`self.SetLifeSpan` _projectiledata_lifetime))