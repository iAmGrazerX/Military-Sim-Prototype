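; Weapon component for the ALS player character, handling semi and full-auto firing, ammo and timed reloads.
; Fire requires ammo, no reload or cooldown, a valid character mesh asset and the aim state.
; It traces from the camera through screen center, spawns BP_ProjectileBase at the muzzle socket toward that target, then starts a cooldown timer.
; Reload refills the magazine from reserve ammo after a delay.
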(event `self.ReceiveBeginPlay`
  ; Casting To Character
  (bind _asals_anim_man_character_bp (cast `/Game/AdvancedLocomotionV4/Blueprints/CharacterLogic/ALS_AnimMan_CharacterBP` (`GameplayStatics.GetPlayerCharacter` 0))
    (:`then`
      (set `self.Character Ref` _asals_anim_man_character_bp))
    (:`CastFailed`
      (`KismetSystemLibrary.PrintString` "Failed to cast Character BP" true true (struct :`R` 1.0 :`G` 0.02598 :`A` 1.0)))))

(fn `CanFire`
  (returns (CanFire :type Boolean))
  (bind _character_ref (`self.Character Ref`))
  (if (!= (or (`self.isReloading`) (<= (`self.CurrentAmmo`) 0) (`self.isOnCooldown`)) true)
    ; Checking Weapon in Hand
    (`/Engine/EditorBlueprintResources/StandardMacros.IsValid` (`SkeletalMeshComponent.GetSkeletalMeshAsset` (`/Game/AdvancedLocomotionV4/Blueprints/CharacterLogic/ALS_AnimMan_CharacterBP.SkeletalMesh` _character_ref))
      (:`Is Valid`
        ; Checking Aim State
        (bind (_pawnmovementmode _movementstate _prevmovementstate _movementaction _rotationmode) (message `/Game/AdvancedLocomotionV4/Blueprints/Interfaces/ALS_Character_BPI.BPI_Get_CurrentStates` _character_ref))
        (if (`|EnumEquality` _rotationmode "NewEnumerator3")
          (return true)
          (else
            (return false)))))))

(fn `FinishedReload`
  (locals (AmmoNeeded :type Integer) (AmmoToReload :type Integer :default 0))
  (bind _output_get (set `local.AmmoNeeded` (- (`self.MaxAmmo`) (`self.CurrentAmmo`))))
  (bind _output_get_2 (set `local.AmmoToReload` (`KismetMathLibrary.Min` _output_get (`self.ReserveAmmo`))))
  (set `self.CurrentAmmo` (+ _output_get_2 (`self.CurrentAmmo`)))
  (set `self.ReserveAmmo` (- (`self.ReserveAmmo`) (`local.AmmoToReload`)))
  (set `self.isReloading` false)
  (set `self.ReloadTimerHandle` (struct))
  (`KismetSystemLibrary.PrintString` "Reloaded!" true false (struct :`R` 0.060735 :`G` 1.0 :`A` 1.0)))

(fn `Fire`
  (bind _returnvalue (`GameplayStatics.GetPlayerController` 0))
  (bind (_sizex _sizey) (`PlayerController.GetViewportSize` _returnvalue))
  (bind _returnvalue_2 (`SceneComponent.GetSocketLocation` (`/Game/AdvancedLocomotionV4/Blueprints/CharacterLogic/ALS_AnimMan_CharacterBP.SkeletalMesh` (`self.Character Ref`)) "muzzle"))
  (bind (_worldposition _worlddirection) (`GameplayStatics.DeprojectScreenToWorld` _returnvalue (`KismetMathLibrary.MakeVector2D` (`KismetMathLibrary.Conv_IntToDouble` (/ _sizex 2)) (`KismetMathLibrary.Conv_IntToDouble` (/ _sizey 2)))))
  (bind _canfire (`self.CanFire`))
  (if _canfire
    (bind _outhit (`KismetSystemLibrary.LineTraceSingle` :`Start` (`PlayerCameraManager.GetCameraLocation` (`GameplayStatics.GetPlayerCameraManager` 0)) :`End` (+ _worldposition (* _worlddirection (`self.Trace Range`))) :`TraceChannel` "TraceTypeQuery1" :`DrawDebugType` "ForDuration" :`DrawTime` 1.0))
    (bind (_bblockinghit _binitialoverlap _time _distance _location _impactpoint _normal _impactnormal _physmat _hitactor _hitcomponent _hitbonename _bonename _hititem _elementindex _faceindex _tracestart _traceend) (`GameplayStatics.BreakHitResult` _outhit))
    ; Setting Target Point based on Trace Hit
    (if _bblockinghit
      (set `self.Target Point` _impactpoint) ; If Line Trace hits an object
      (else
        (set `self.Target Point` _traceend) ; If Line trace doesn't hit anything
      ))
    ; Spawning Projectile & Setting it's data
    (`|SpawnActorFromClass` "/Game/MyContent/Weapon/Blueprint/BP_ProjectileBase.BP_ProjectileBase_C" (`KismetMathLibrary.MakeTransform` _returnvalue_2 (`KismetMathLibrary.FindLookAtRotation` _returnvalue_2 (`self.Target Point`))) "Undefined" "MultiplyWithRoot" null (`self.WeaponProjectileData`) (`self.Character Ref`))
    (`/Engine/EditorBlueprintResources/StandardMacros.DecrementInt` (`self.CurrentAmmo`)
      (:`  `
        ; Handling Cooldown between shots
        (set `self.isOnCooldown` true)
        (bind _returnvalue_3 (`KismetSystemLibrary.K2_SetTimer` null "ResetCooldown" (`self.FireRate`)))
        (set `self.FireTimerHandle` _returnvalue_3)))))

(fn `Reload`
  (if (or (`self.isReloading`) (>= (`self.CurrentAmmo`) (`self.MaxAmmo`)))
    (return)
    (else
      (set `self.isReloading` true)
      (`KismetSystemLibrary.PrintString` "Reloading" true false (struct :`R` 0.060735 :`G` 1.0 :`A` 1.0))
      (bind _returnvalue (`KismetSystemLibrary.K2_SetTimer` null "FinishedReload" (`self.ReloadTime`)))
      (set `self.ReloadTimerHandle` _returnvalue))))

(fn `ResetCooldown`
  (set `self.isOnCooldown` false))

(fn `Start Fire`
  (switch `/Game/MyContent/Weapon/Enum/E_FireMode` (`self.FireMode`)
    (:`NewEnumerator1`
      (`self.Fire`))
    (:`NewEnumerator0`
      (set `self.IsFiring` true)
      (bind _returnvalue (`KismetSystemLibrary.K2_SetTimerDelegate` :`Time` (`self.FireRate`) :`bLooping` true))
      (set `self.FireTimerHandle` _returnvalue)
      (`self.Fire`))))

(fn `Stop Fire`
  (set `self.IsFiring` false)
  (set `self.FireTimerHandle` (struct)))